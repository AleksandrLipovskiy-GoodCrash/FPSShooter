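; Assault rifle weapon Blueprint that adds automatic fire to a parent weapon class.
; BeginPlay pulls its ammo data from the FPS game instance.
; Firing starts a looping timer that calls the parent fire logic, plays the gun animation, spawns shell-eject particles and notifies the owning character.
; An empty magazine stops fire and triggers the character's reload; stopping clears the timer.
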(event Custom|StartRifleFire
  (bind _gun (Variables|Default|GetGun))
  (bind _returnvalue (Transformation|GetSocketTransform _gun "AmmoEject" "RTS_World"))
  (if (Variables|Default|GetisRifleFiring)
    (|CallParentFunction (stale EventWeaponFire FireType))
    (Components|Animation|PlayAnimation (Variables|Default|GetGun) "/Game/Weapons/Weapons/Anims/Fire_Rifle_W.Fire_Rifle_W" false)
    (Effects|SpawnEmitteratLocation "/Game/Effects/Particles/FX_AssauilRifleShell.FX_AssauilRifleShell" (.location _returnvalue) (.rotation _returnvalue))
    (Default|CallCharacterFireWeapon (Variables|Default|GetMainCharacterRef) "NewEnumerator1")
    (if (<= (Variables|Default|GetCurrentAmmoInMag) 0)
      (CallFunction|StopFire)
      (Default|ReloadWeapon (Variables|Default|GetMainCharacterRef)))))

(event EventBeginPlay
  (|CallParentFunction)
  (bind _asfps_game_instance_bp (Utilities|Casting|CastToFPS_GameInstance_BP (Game|GetGameInstance)))
  (Variables|Default|SetAmmoData (Variables|/Game/Blueprints/FPS_GameInstance_BP.FPS_GameInstance_BP_C|GetAssaultRifleAmmoData _asfps_game_instance_bp)))

(event Collision|EventActorBeginOverlap
  (params (OtherActor :type Actor%20Object%20Reference))
  (|CallParentFunction OtherActor) ; This node is disabled and will not be called.\nDrag off pins to build functionality.
)

(event EventTick
  (params (DeltaSeconds :type Float%20%28single-precision%29))
  (|CallParentFunction DeltaSeconds) ; This node is disabled and will not be called.\nDrag off pins to build functionality.
)

(event EventWeaponFire
  (params (FireType :type FireTypeEnum_BP%20Enum :default "NewEnumerator0"))
  (Variables|Default|SetisRifleFiring true)
  (CallFunction|StartRifleFire)
  (bind _returnvalue (Utilities|Time|SetTimerbyEvent (delegate Custom|StartRifleFire) (Variables|Default|GetAutomaticFireRate) true))
  (Variables|Default|SetRifleFireTimerHandle _returnvalue))

(event EventStopFire
  (|CallParentFunction)
  (Variables|Default|SetisRifleFiring false)
  (Utilities|Time|ClearandInvalidateTimerbyHandle (Variables|Default|GetRifleFireTimerHandle)))

(fn ConstructionScript
  (|CallParentFunction))