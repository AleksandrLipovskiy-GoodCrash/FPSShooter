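; Rocket launcher weapon Blueprint that extends a parent weapon class with launcher-specific ammo data and fire feedback.
; On BeginPlay it pulls its ammo data from the RocketLauncherAmmoData entry in the FPS game instance.
; WeaponFire runs the parent logic, then plays the launcher's gun fire animation and a world camera shake centered on the weapon.
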(event EventBeginPlay
  (|CallParentFunction)
  (bind _asfps_game_instance_bp (Utilities|Casting|CastToFPS_GameInstance_BP (Game|GetGameInstance)))
  (Variables|Default|SetAmmoData (Variables|/Game/Blueprints/FPS_GameInstance_BP.FPS_GameInstance_BP_C|GetRocketLauncherAmmoData _asfps_game_instance_bp)))

(event EventWeaponFire
  (params (FireType :type FireTypeEnum_BP%20Enum :default "NewEnumerator0"))
  (|CallParentFunction FireType)
  (Components|Animation|PlayAnimation (Variables|Default|GetGun) "/Game/Weapons/Weapons/Anims/Fire_RocketLauncher_W.Fire_RocketLauncher_W" false)
  (Camera|PlayWorldCameraShake "/Game/Blueprints/CameraShakes/RocketLauncherCameraShake_BP.RocketLauncherCameraShake_BP_C" (Transformation|GetActorLocation) 0.0 5e+02))

(fn ConstructionScript
  (|CallParentFunction))