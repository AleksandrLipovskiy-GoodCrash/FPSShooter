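; Pistol weapon Blueprint that extends a parent weapon class with pistol-specific ammo data and firing effects.
; On BeginPlay it copies the pistol ammo data from the FPS game instance into its own AmmoData.
; Firing runs the parent logic, then plays the gun's fire animation and spawns a shell particle at the AmmoEject socket.
; Reload and construction defer entirely to the parent.
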(event EventBeginPlay
  (|CallParentFunction)
  (bind _asfps_game_instance_bp (Utilities|Casting|CastToFPS_GameInstance_BP (Game|GetGameInstance)))
  (Variables|Default|SetAmmoData (Variables|/Game/Blueprints/FPS_GameInstance_BP.FPS_GameInstance_BP_C|GetPistolAmmoData _asfps_game_instance_bp)))

(event Collision|EventActorBeginOverlap
  (params (OtherActor :type Actor%20Object%20Reference))
  (|CallParentFunction OtherActor) ; This node is disabled and will not be called.\nDrag off pins to build functionality.
)

(event EventTick
  (params (DeltaSeconds :type Float%20%28single-precision%29))
  (|CallParentFunction DeltaSeconds) ; This node is disabled and will not be called.\nDrag off pins to build functionality.
)

(event EventWeaponFire
  (params (FireType :type FireTypeEnum_BP%20Enum :default "NewEnumerator0"))
  (bind _gun (Variables|Default|GetGun))
  (bind _returnvalue (Transformation|GetSocketTransform _gun "AmmoEject" "RTS_World"))
  (|CallParentFunction FireType)
  (Components|Animation|PlayAnimation (Variables|Default|GetGun) "/Game/Weapons/Weapons/Anims/Fire_Pistol_W.Fire_Pistol_W" false)
  (Effects|SpawnEmitteratLocation "/Game/Effects/Particles/FX_PistolShell.FX_PistolShell" (.location _returnvalue) (.rotation _returnvalue)))

(event EventWeaponReload
  (|CallParentFunction))

(fn ConstructionScript
  (|CallParentFunction))