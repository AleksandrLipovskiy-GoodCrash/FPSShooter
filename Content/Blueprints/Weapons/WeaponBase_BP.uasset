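; Base weapon Blueprint for the FPS character, handling firing, magazine ammo, reloading and aim state.
; WeaponFire traces from the camera, adding random spread unless aiming, for single or multi-bullet hitscan with impact effects and damage messages, or projectiles.
; Projectiles launch from the muzzle socket toward the traced point, falling back to control rotation.
; Automatic weapons play a reversing timeline for controller recoil, while Tick updates the character's ADS FOV.
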(event Custom|ControllerInputRecoil
  (bind _returnvalue (Game|Player|GetPlayerPawn 0))
  (bind (_direction _alpha) (Timeline|AutomaticRecoilTimeline PlayFromStart)
    (:Update
      (switch Utilities|FlowControl|Switch|SwitchonETimelineDirection _direction
        (:Forward
          (Pawn|Input|AddControllerPitchInput _returnvalue (Math|Float|Lerp 0.0 (Variables|Recoil|GetRecoilPitch) _alpha))
          (Pawn|Input|AddControllerYawInput _returnvalue (Math|Random|RandomFloatinRange -0.15 0.15)))
        (:Backward
          (Pawn|Input|AddControllerPitchInput (Game|Player|GetPlayerPawn 0) (* (Math|Float|Lerp 0.0 (Variables|Recoil|GetRecoilPitch) _alpha) -1.0)))))
    (:Finished
      (CallFunction|ReverseRecoil)
      (Utilities|FlowControl|RetriggerableDelay 0.05)
      (CallFunction|StopRecoil))))

(event Custom|StopRecoil
  (bind _returnvalue (Game|Player|GetPlayerPawn 0))
  (bind (_direction _alpha) (Timeline|AutomaticRecoilTimeline Stop)
    (:Update
      (switch Utilities|FlowControl|Switch|SwitchonETimelineDirection _direction
        (:Forward
          (Pawn|Input|AddControllerPitchInput _returnvalue (Math|Float|Lerp 0.0 (Variables|Recoil|GetRecoilPitch) _alpha))
          (Pawn|Input|AddControllerYawInput _returnvalue (Math|Random|RandomFloatinRange -0.15 0.15)))
        (:Backward
          (Pawn|Input|AddControllerPitchInput (Game|Player|GetPlayerPawn 0) (* (Math|Float|Lerp 0.0 (Variables|Recoil|GetRecoilPitch) _alpha) -1.0)))))
    (:Finished
      (CallFunction|ReverseRecoil)
      (Utilities|FlowControl|RetriggerableDelay 0.05)
      (CallFunction|StopRecoil))))

(event Custom|ReverseRecoil
  (bind _returnvalue (Game|Player|GetPlayerPawn 0))
  (bind (_direction _alpha) (Timeline|AutomaticRecoilTimeline Reverse)
    (:Update
      (switch Utilities|FlowControl|Switch|SwitchonETimelineDirection _direction
        (:Forward
          (Pawn|Input|AddControllerPitchInput _returnvalue (Math|Float|Lerp 0.0 (Variables|Recoil|GetRecoilPitch) _alpha))
          (Pawn|Input|AddControllerYawInput _returnvalue (Math|Random|RandomFloatinRange -0.15 0.15)))
        (:Backward
          (Pawn|Input|AddControllerPitchInput (Game|Player|GetPlayerPawn 0) (* (Math|Float|Lerp 0.0 (Variables|Recoil|GetRecoilPitch) _alpha) -1.0)))))
    (:Finished
      (CallFunction|ReverseRecoil)
      (Utilities|FlowControl|RetriggerableDelay 0.05)
      (CallFunction|StopRecoil))))

(event Custom|OnAimEnter
  (Variables|ADS|SetisAiming true))

(event Custom|OnAimExit
  (Variables|ADS|SetisAiming false))

(event EventBeginPlay
  (bind _asfps_main_character_bp (Utilities|Casting|CastToFPS_MainCharacter_BP (Game|Player|GetPlayerPawn 0)))
  (Variables|References|SetMainCharacterRef _asfps_main_character_bp)
  (EventDispatchers|AssignAimEnter _asfps_main_character_bp (delegate Custom|OnAimEnter))
  (EventDispatchers|AssignAimExit _asfps_main_character_bp (delegate Custom|OnAimExit)))

(event EventTick
  (params (DeltaSeconds :type Float%20%28single-precision%29))
  (Default|SetADSFOV (Variables|References|GetMainCharacterRef)))

(fn ConstructionScript)

(fn WeaponFire
  (params (FireType :type FireTypeEnum_BP%20Enum :default "NewEnumerator0"))
  (Variables|Ammo|SetCurrentAmmoInMag (- (Variables|Ammo|GetCurrentAmmoInMag) 1))
  (switch Utilities|FlowControl|Switch|SwitchonFireTypeEnum_BP FireType
    (:NewEnumerator0
      (if (Variables|Ammo|GetisMultipleBullets)
        (for _index (range 0 (- (Variables|Ammo|GetBulletCount) 1))
          (bind _hitresult (CallFunction|CalculateShot (Variables|/Game/Blueprints/FPS_MainCharacter_BP.FPS_MainCharacter_BP_C|GetCamera (Variables|References|GetMainCharacterRef)) (Variables|Default|GetGun) "MuzzleFlash"))
          (Game|SpawnActorfromClass (Variables|WeaponProps|GetImpactEffectClass) (Math|Transform|MakeTransform (.ImpactPoint (Collision|BreakHitResult _hitresult)) "0, 0, 0" "1,1,1") "Undefined" 0 _hitresult (.bBlockingHit (Collision|BreakHitResult _hitresult)) 0)
          (CallFunction|AddDamage _hitresult)
          (if (Variables|WeaponProps|GetisAutomaticWeapon)
            (CallFunction|ControllerInputRecoil)))
        (else
          (bind _hitresult_2 (CallFunction|CalculateShot (Variables|/Game/Blueprints/FPS_MainCharacter_BP.FPS_MainCharacter_BP_C|GetCamera (Variables|References|GetMainCharacterRef)) (Variables|Default|GetGun) "MuzzleFlash"))
          (Game|SpawnActorfromClass (Variables|WeaponProps|GetImpactEffectClass) (Math|Transform|MakeTransform (.ImpactPoint (Collision|BreakHitResult _hitresult_2)) "0, 0, 0" "1,1,1") "Undefined" 0 _hitresult_2 (.bBlockingHit (Collision|BreakHitResult _hitresult_2)) 0)
          (CallFunction|AddDamage _hitresult_2)
          (if (Variables|WeaponProps|GetisAutomaticWeapon) :!label _label
            (CallFunction|ControllerInputRecoil)))))
    (:NewEnumerator1
      (bind _projectiletransform (CallFunction|CalculateShot (Variables|/Game/Blueprints/FPS_MainCharacter_BP.FPS_MainCharacter_BP_C|GetCamera (Variables|References|GetMainCharacterRef)) (Variables|Default|GetGun) "MuzzleFlash"))
      (bind _returnvalue (Game|SpawnActorfromClass (Variables|Projectile|GetProjectile) _projectiletransform "AlwaysSpawn" 0 (Variables|WeaponProps|GetAmmoData) (Variables|Stats|GetCriticalHitDamageModifier) 0))
      (Variables|Projectile|SetSpawnedProjectile _returnvalue)
      (goto _label))))

(fn WeaponReload
  (Variables|Ammo|SetCurrentAmmoInMag (Math|Integer|Min(Integer) (Variables|Ammo|GetMaxMagAmmo) (Variables|Ammo|GetCurrentTotalAmmo)))
  (Variables|Ammo|SetCurrentTotalAmmo (- (Variables|Ammo|GetCurrentTotalAmmo) (Math|Integer|Min(Integer) (Variables|Ammo|GetMaxMagAmmo) (Variables|Ammo|GetCurrentTotalAmmo)))))

(fn HasAmmoinMag
  (return (> (Variables|Ammo|GetCurrentAmmoInMag) 0) (== (Variables|Ammo|GetCurrentAmmoInMag) (Variables|Ammo|GetMaxMagAmmo))))

(fn HasExtraAmmo
  (return (> (Variables|Ammo|GetCurrentTotalAmmo) 0)))

(fn CalculateShot
  (params (Camare :type Camera%20Component%20Object%20Reference) (WeaponMesh :type Scene%20Component%20Object%20Reference) (WeaponFireSocketName :type Name))
  (Utilities|FlowControl|Sequence
    (:then_0
      (LocalVariables|SetLocalCamera Camare)
      (LocalVariables|SetLocalWeaponMesh WeaponMesh)
      (LocalVariables|SetLocalWeaponFireSocketName WeaponFireSocketName))
    (:then_1
      (bind (_outhit _returnvalue) (Collision|LineTraceForObjects (.Start (CallFunction|GetStartEndLineTraceforShot (LocalVariables|GetLocalCamera) (Variables|Stats|GetBulletSpread))) (.End (CallFunction|GetStartEndLineTraceforShot (LocalVariables|GetLocalCamera) (Variables|Stats|GetBulletSpread))) (Utilities|Array|MakeArray "ObjectTypeQuery1" "ObjectTypeQuery2") false (Utilities|Array|MakeArray (Game|Player|GetPlayerPawn 0)) "None"))
      (if _returnvalue
        (LocalVariables|SetLocalProjectileTransform (Math|Transform|MakeTransform (Transformation|GetSocketLocation (LocalVariables|GetLocalWeaponMesh) (LocalVariables|GetLocalWeaponFireSocketName)) (Math|Rotator|FindLookatRotation (Transformation|GetSocketLocation (LocalVariables|GetLocalWeaponMesh) (LocalVariables|GetLocalWeaponFireSocketName)) (.ImpactPoint (Collision|BreakHitResult _outhit)))))
        (else
          (LocalVariables|SetLocalProjectileTransform (Math|Transform|MakeTransform (Transformation|GetSocketLocation (LocalVariables|GetLocalWeaponMesh) (LocalVariables|GetLocalWeaponFireSocketName)) (Pawn|GetControlRotation (.AsPawn (Utilities|Casting|CastToPawn (Components|GetOwner (LocalVariables|GetLocalCamera)))) :!class /Script/Engine.Pawn))))))
    (:then_2
      (return _outhit (LocalVariables|GetLocalProjectileTransform)))))

(fn GetStartEndLineTraceforShot
  (params (Camera :type Camera%20Component%20Object%20Reference) (BulletSpread :type Float%20%28single-precision%29))
  (bind _returnvalue (Transformation|GetWorldTransform Camera))
  (bind _returnvalue_2 (* BulletSpread -1.0))
  (bind _returnvalue_3 (Math|Vector|GetForwardVector (.rotation _returnvalue)))
  (bind _returnvalue_4 (* _returnvalue_3 1e+04))
  (bind _returnvalue_5 (+ (.location _returnvalue) _returnvalue_4))
  (bind (_x _y _z) (Math|Vector|BreakVector _returnvalue_5))
  (return (.location _returnvalue) (select (Variables|ADS|GetisAiming) _returnvalue_5 (Math|Vector|MakeVector (+ _x (Math|Random|RandomFloatinRange _returnvalue_2 BulletSpread)) (+ _y (Math|Random|RandomFloatinRange _returnvalue_2 BulletSpread)) (+ _z (Math|Random|RandomFloatinRange _returnvalue_2 BulletSpread))))))

(fn AddDamage
  (params (HitResult :type Hit%20Result%20Structure))
  (Class|TakeDamageBP|TakeDamage(Message) (.HitActor (Collision|BreakHitResult HitResult)) (Variables|WeaponProps|GetAmmoData) (Variables|Stats|GetCriticalHitDamageModifier) HitResult))

(fn StopFire)