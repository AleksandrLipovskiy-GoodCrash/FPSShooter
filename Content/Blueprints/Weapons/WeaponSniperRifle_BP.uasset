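; Sniper rifle weapon Blueprint, a child weapon that loads its ammo data from the game instance.
; Firing plays the gun animation, then applies controller recoil when aiming or ejects a shell effect when not.
; Aiming blocks weapon switching and reloading, then after a short delay shows a scope HUD and hides the gun, player pawn and main HUD.
; Exiting aim reverses these changes.
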(event EventBeginPlay
  (|CallParentFunction)
  (bind _asfps_game_instance_bp (Utilities|Casting|CastToFPS_GameInstance_BP (Game|GetGameInstance)))
  (Variables|Default|SetAmmoData (Variables|/Game/Blueprints/FPS_GameInstance_BP.FPS_GameInstance_BP_C|GetSniperRifleAmmoData _asfps_game_instance_bp)))

(event EventWeaponFire
  (params (FireType :type FireTypeEnum_BP%20Enum :default "NewEnumerator0"))
  (bind _gun (Variables|Default|GetGun))
  (bind _returnvalue (Transformation|GetSocketTransform _gun "AmmoEject" "RTS_World"))
  (|CallParentFunction FireType)
  (Components|Animation|PlayAnimation (Variables|Default|GetGun) "/Game/Weapons/Weapons/Anims/Fire_SniperRifle_W.Fire_SniperRifle_W" false)
  (if (Variables|Default|GetisAiming)
    (CallFunction|ControllerInputRecoil)
    (else
      (Effects|SpawnEmitteratLocation "/Game/Effects/Particles/FX_SniperRifleShell.FX_SniperRifleShell" (.location _returnvalue) (.rotation _returnvalue)))))

(event EventOnAimEnter
  (bind _maincharacterref (Variables|Default|GetMainCharacterRef))
  (bind _maincharacterref_2 (Variables|Default|GetMainCharacterRef))
  (bind _sniperscopehudref (Variables|/Game/Blueprints/FPS_MainCharacter_BP.FPS_MainCharacter_BP_C|GetSniperScopeHUDRef _maincharacterref_2))
  (|CallParentFunction)
  (if (== (Variables|/Game/Blueprints/FPS_MainCharacter_BP.FPS_MainCharacter_BP_C|GetCurrentWeapon (Variables|Default|GetMainCharacterRef)) self)
    (Variables|/Game/Blueprints/FPS_MainCharacter_BP.FPS_MainCharacter_BP_C|SetisCanSwitchweapon _maincharacterref false)
    (Variables|/Game/Blueprints/FPS_MainCharacter_BP.FPS_MainCharacter_BP_C|SetisCanReload _maincharacterref false)
    (Utilities|FlowControl|Delay 0.1)
    (if (not (UserInterface|Viewport|IsinViewport _sniperscopehudref))
      (UserInterface|Viewport|AddtoViewport _sniperscopehudref 0)
      (Development|SetHiddeninGame (Variables|Default|GetGun) true false)
      (Rendering|SetActorHiddenInGame (Game|Player|GetPlayerPawn 0) true)
      (Widget|SetVisibility (Variables|/Game/Blueprints/FPS_MainCharacter_BP.FPS_MainCharacter_BP_C|GetMainHUDRef (Variables|Default|GetMainCharacterRef)) "Collapsed"))))

(event EventOnAimExit
  (bind _maincharacterref (Variables|Default|GetMainCharacterRef))
  (|CallParentFunction)
  (Variables|/Game/Blueprints/FPS_MainCharacter_BP.FPS_MainCharacter_BP_C|SetisCanSwitchweapon _maincharacterref true)
  (Variables|/Game/Blueprints/FPS_MainCharacter_BP.FPS_MainCharacter_BP_C|SetisCanReload _maincharacterref true)
  (Widget|RemovefromParent (Variables|/Game/Blueprints/FPS_MainCharacter_BP.FPS_MainCharacter_BP_C|GetSniperScopeHUDRef _maincharacterref))
  (Development|SetHiddeninGame (Variables|Default|GetGun) false false)
  (Rendering|SetActorHiddenInGame (Game|Player|GetPlayerPawn 0) false)
  (Widget|SetVisibility (Variables|/Game/Blueprints/FPS_MainCharacter_BP.FPS_MainCharacter_BP_C|GetMainHUDRef (Variables|Default|GetMainCharacterRef)) "Visible"))

(fn ConstructionScript
  (|CallParentFunction))