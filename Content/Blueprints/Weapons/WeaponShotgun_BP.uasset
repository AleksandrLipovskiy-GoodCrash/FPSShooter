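; Shotgun weapon Blueprint that extends a parent weapon class with shotgun-specific ammo, reload timing and firing effects.
; On BeginPlay it pulls its ammo data from the FPS game instance, then derives reload time from magazine capacity.
; Firing runs the parent logic, then plays the gun's fire animation and spawns a shell-eject particle at the AmmoEject socket.
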(event Custom|SetReloadTime
  (Variables|Default|SetReloadTime (* (Variables|Default|GetMaxMagAmmo) 0.5)))

(event EventBeginPlay
  (|CallParentFunction)
  (bind _asfps_game_instance_bp (Utilities|Casting|CastToFPS_GameInstance_BP (Game|GetGameInstance)))
  (Variables|Default|SetAmmoData (Variables|/Game/Blueprints/FPS_GameInstance_BP.FPS_GameInstance_BP_C|GetShotgunAmmoData _asfps_game_instance_bp))
  (CallFunction|SetReloadTime))

(event Collision|EventActorBeginOverlap
  (params (OtherActor :type Actor%20Object%20Reference)))

(event EventTick
  (params (DeltaSeconds :type Float%20%28single-precision%29)))

(event EventWeaponFire
  (params (FireType :type FireTypeEnum_BP%20Enum :default "NewEnumerator0"))
  (bind _gun (Variables|Default|GetGun))
  (bind _returnvalue (Transformation|GetSocketTransform _gun "AmmoEject" "RTS_World"))
  (|CallParentFunction FireType)
  (Components|Animation|PlayAnimation (Variables|Default|GetGun) "/Game/Weapons/Weapons/Anims/Fire_Shotgun_W.Fire_Shotgun_W" false)
  (Effects|SpawnEmitteratLocation "/Game/Effects/Particles/FX_ShotgunShell.FX_ShotgunShell" (.location _returnvalue) (.rotation _returnvalue)))

(fn ConstructionScript
  (|CallParentFunction))