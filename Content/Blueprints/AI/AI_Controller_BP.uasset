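; AI controller that runs AI_BehaviorTree on BeginPlay and caches its controlled pawn as an AI_CharacterBase_BP.
; On perception updates, it passes each updated actor's last sensed stimuli to AISense.
; AISense handles only stimulus index 0, writing its success flag to the isCanSeePlayer Blackboard key.
; The sense is identified by array position, and nothing checks that the sensed actor is the player.
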(event OnPerceptionUpdated(AIPerception)
  (params (UpdatedActors :type Array%20of%20Actor%20Object%20References))
  (for _array_element UpdatedActors
    (bind _info (Class|AIPerceptionComponent|GetActorsPerception (Variables|Default|GetAIPerception) _array_element))
    (CallFunction|AISense (.lastsensedstimuli _info))))

(event EventBeginPlay
  (AI|RunBehaviorTree "/Game/Blueprints/AI/AI_BehaviorTree.AI_BehaviorTree")
  (bind _asai_character_base_bp (Utilities|Casting|CastToAI_CharacterBase_BP (Pawn|GetControlledPawn)))
  (Variables|Default|SetAI_CharacterRef _asai_character_base_bp))

(fn ConstructionScript)

(fn AISense
  (params (AIStimulus :type Array%20of%20AI%20Stimulus%20Structures))
  (for (_array_element _array_index) AIStimulus
    (LocalVariables|SetCurrentSense _array_element)
    (switch int _array_index
      (:0
        (AI|Components|Blackboard|SetValueasBool (AI|GetBlackboard 0) (Utilities|Name|MakeLiteralName "isCanSeePlayer") (.bSuccessfullySensed (Utilities|Struct|BreakAIStimulus (LocalVariables|GetCurrentSense))))))))