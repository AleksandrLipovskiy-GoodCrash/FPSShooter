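; Base AI character that takes player weapon damage, dies, and plays a zombie melee attack montage.
; Direct hits apply a random critical roll and physical-material multiplier, while radius hits fall off linearly with distance.
; Both report damage to AI sense, update health, and spawn floating damage and hitmarker widgets.
; Death sets the blackboard isDead key and ragdolls the mesh with an impulse away from the player, scaled by weapon.
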(event EventTakeDamageRadius
  (params (GroundHitResult :type Hit%20Result%20Structure) (AmmoData :type Ammo%20Data%20BP%20Structure) (CriticalHitDamageModifier :type Float%20%28single-precision%29))
  (bind (_damage _criticalhitchance _damageradius) (Utilities|Struct|BreakAmmoData_BP AmmoData))
  (bind (_bblockinghit _binitialoverlap _time _distance _location _impactpoint _normal _impactnormal _physmat _hitactor _hitcomponent _hitbonename) (Collision|BreakHitResult GroundHitResult))
  (if (not (Variables|Default|GetisDead))
    (bind _damagetoapply (CallFunction|SetDamageRadius _damage 0.0 _damageradius _impactpoint))
    (Class|AISenseDamage|ReportDamageEvent self (Game|GetPlayerCharacter 0) _damagetoapply _impactpoint)
    (bind _isdead (CallFunction|UpdateHealth _damagetoapply))
    (bind _output_get (Variables|Default|SetisDead _isdead))
    (if _output_get
      (CallFunction|Die _impactpoint _hitbonename))
    (CallFunction|FloatingDamage _damagetoapply _impactpoint)
    (Utilities|IsValid (Variables|Default|GetUI_HitmarkerRef)
      (:Is%20Valid
        (Widget|RemovefromParent (Variables|Default|GetUI_HitmarkerRef)))
      (:Is%20Not%20Valid
        _))
    (bind _returnvalue (UserInterface|CreateWidget "/Game/Blueprints/UMG/UI_Hitmarker_BP.UI_Hitmarker_BP_C" 0 (Variables|Default|GetisDead)))
    (bind _output_get_2 (Variables|Default|SetUI_HitmarkerRef _returnvalue))
    (UserInterface|Viewport|AddtoViewport _output_get_2 0)))

(event EventFloatingDamage
  (params (DamageValue :type Float%20%28single-precision%29) (ImpactPoint :type Vector :default "0, 0, 0"))
  (bind _returnvalue (Game|GetPlayerController 0))
  (bind _screenposition (Class|WidgetLayoutLibrary|ProjectWorldLocationtoWidgetPosition _returnvalue ImpactPoint false))
  (bind (_x _y) (Math|Vector2D|BreakVector2D _screenposition))
  (bind _returnvalue_2 (UserInterface|CreateWidget "/Game/Blueprints/UMG/UI_FloatingDamage_BP.UI_FloatingDamage_BP_C" 0 DamageValue))
  (Class|Widget|SetRenderTranslation (Variables|/Game/Blueprints/UMG/UI_FloatingDamage_BP.UI_FloatingDamage_BP_C|GetScreenPositionSizeBox _returnvalue_2) (Math|Vector2D|MakeVector2D (+ (+ _x -5e+01) (Math|Random|RandomFloatinRange -25.0 25.0)) (+ (+ _y -1e+02) (Math|Random|RandomFloatinRange -1e+01 1e+01))))
  (UserInterface|Viewport|AddtoViewport _returnvalue_2 0))

(event EventBeginPlay
  (bind _asfps_main_character_bp (Utilities|Casting|CastToFPS_MainCharacter_BP (Game|Player|GetPlayerPawn 0)))
  (Variables|Default|SetMainCharacterRef _asfps_main_character_bp))

(event EventTakeDamage
  (params (AmmoData :type Ammo%20Data%20BP%20Structure) (CriticalHitDamageModifier :type Float%20%28single-precision%29) (HitResult :type Hit%20Result%20Structure))
  (bind (_damage _criticalhitchance) (Utilities|Struct|BreakAmmoData_BP AmmoData))
  (bind (_bblockinghit _binitialoverlap _time _distance _location _impactpoint _normal _impactnormal _physmat _hitactor _hitcomponent _hitbonename) (Collision|BreakHitResult HitResult))
  (if (not (Variables|Default|GetisDead))
    (bind _damagetoapply (CallFunction|SetDamage _damage _criticalhitchance CriticalHitDamageModifier HitResult))
    (Class|AISenseDamage|ReportDamageEvent self (Game|GetPlayerCharacter 0) _damagetoapply _impactpoint)
    (bind _isdead (CallFunction|UpdateHealth _damagetoapply))
    (bind _output_get (Variables|Default|SetisDead _isdead))
    (if _output_get
      (CallFunction|Die _impactpoint _hitbonename))
    (CallFunction|FloatingDamage _damagetoapply _impactpoint)
    (Utilities|IsValid (Variables|Default|GetUI_HitmarkerRef)
      (:Is%20Valid
        (Widget|RemovefromParent (Variables|Default|GetUI_HitmarkerRef)))
      (:Is%20Not%20Valid
        _))
    (bind _returnvalue (UserInterface|CreateWidget "/Game/Blueprints/UMG/UI_Hitmarker_BP.UI_Hitmarker_BP_C" 0 (Variables|Default|GetisDead)))
    (bind _output_get_2 (Variables|Default|SetUI_HitmarkerRef _returnvalue))
    (UserInterface|Viewport|AddtoViewport _output_get_2 0)))

(event EventMeleeAttack
  (Animation|Montage|PlayMontage (Variables|Character|GetMesh) "/Game/Characters/Enemies/ZombieDerrick/Animations/Zombie_Attack_Montage.Zombie_Attack_Montage"))

(fn ConstructionScript)

(fn SetDamage
  (params (DamageValue :type Float%20%28single-precision%29) (CriticalHitChance :type Float%20%28single-precision%29) (CriticalHitDamageModifier :type Float%20%28single-precision%29) (HitResult :type Hit%20Result%20Structure))
  (LocalVariables|SetLocalDomageValue DamageValue)
  (Utilities|FlowControl|Sequence
    (:then_0
      (bind _output_get (LocalVariables|SetLocalIsCriticalHit (< CriticalHitChance (Math|Random|RandomFloatinRange 0.0 1e+02))))
      (if _output_get
        (LocalVariables|SetLocalDomageValue (* (LocalVariables|GetLocalDomageValue) CriticalHitDamageModifier))))
    (:then_1
      (LocalVariables|SetLocalDomageValue (* (LocalVariables|GetLocalDomageValue) (Variables|/Script/PhysicsCore.PhysicalMaterial|GetDestructibleDamageThresholdScale (.PhysMat (Collision|BreakHitResult HitResult))))))
    (:then_2
      (return (LocalVariables|GetLocalDomageValue) (LocalVariables|GetLocalIsCriticalHit)))))

(fn UpdateHealth
  (params (DamageValue :type Float%20%28single-precision%29))
  (Utilities|FlowControl|Sequence
    (:then_0
      (if (>= DamageValue (Variables|Default|GetCurrentHealth))
        (LocalVariables|SetLocalIsDead true)
        (Variables|Default|SetCurrentHealth 0.0)
        (else
          (Variables|Default|SetCurrentHealth (- (Variables|Default|GetCurrentHealth) DamageValue)))))
    (:then_1
      (return (LocalVariables|GetLocalIsDead)))))

(fn SetDamageRadius
  (params (DamageValue :type Float%20%28single-precision%29) (CriticalHitChance :type Float%20%28single-precision%29) (Radius :type Float%20%28single-precision%29) (GroundPoint :type Vector))
  (LocalVariables|SetLocalDomageValue DamageValue)
  (Utilities|FlowControl|Sequence
    (:then_0
      (LocalVariables|SetLocalIsCriticalHit (< CriticalHitChance (Math|Random|RandomFloatinRange 0.0 1e+02))))
    (:then_1
      (return (Math|Float|Clamp(Float) (* (- 1.0 (/ (Math|Vector|VectorLength (- GroundPoint (Transformation|GetActorLocation))) Radius)) (LocalVariables|GetLocalDomageValue)) 0.0 (LocalVariables|GetLocalDomageValue)) (LocalVariables|GetLocalIsCriticalHit)))))

(fn Die
  (params (ImpactPoint :type Vector) (BoneName :type Name))
  (bind _mesh (Variables|Character|GetMesh))
  (bind _maincharacterref (Variables|Default|GetMainCharacterRef))
  (AI|Components|Blackboard|SetValueasBool (AI|GetBlackboard (Pawn|GetController)) (Utilities|Name|MakeLiteralName "isDead") true)
  (Physics|SetSimulatePhysics _mesh true)
  (Physics|AddImpulseatLocation _mesh (* (Math|Vector|GetUnitDirection(Vector) (Transformation|GetActorLocation _maincharacterref) (Transformation|GetActorLocation)) (Utilities|Select :Index (Variables|/Game/Blueprints/FPS_MainCharacter_BP.FPS_MainCharacter_BP_C|GetHasWeaponEquipedEnum _maincharacterref) :NewEnumerator0 1e+04 :NewEnumerator1 (Variables|/Game/Blueprints/Weapons/WeaponBase_BP.WeaponBase_BP_C|GetKillImpulse (Variables|/Game/Blueprints/FPS_MainCharacter_BP.FPS_MainCharacter_BP_C|GetCurrentWeapon _maincharacterref)))) ImpactPoint BoneName))