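; First-person shooter player controller that turns the TurnRight and TurnUp axis inputs into yaw and pitch look input.
; On BeginPlay it caches the pawn of player 0 as an FPS_MainCharacter_BP reference.
; Both axes cut sensitivity to a third while that character is aiming with one specific equipped-weapon enum value, and pass input through unchanged otherwise.
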(event EventBeginPlay
  (bind _asfps_main_character_bp (Utilities|Casting|CastToFPS_MainCharacter_BP (Game|Player|GetPlayerPawn 0)))
  (Variables|Default|SetMainCharacterRef _asfps_main_character_bp))

(event Input|AxisEvents|InputAxisTurnRight
  (params (AxisValue :type Float%20%28single-precision%29))
  (bind _maincharacterref (Variables|Default|GetMainCharacterRef))
  ;[1 1 1] Turn Right/Left
  (Class|PlayerController|AddYawInput (select (and (Variables|/Game/Blueprints/FPS_MainCharacter_BP.FPS_MainCharacter_BP_C|GetisAiming _maincharacterref) (Utilities|Enum|Equal(Enum) (Variables|/Game/Blueprints/FPS_MainCharacter_BP.FPS_MainCharacter_BP_C|GetHasWeaponEquipedEnum _maincharacterref) "NewEnumerator1")) (/ AxisValue 3.0) AxisValue)))

(event Input|AxisEvents|InputAxisTurnUp
  (params (AxisValue :type Float%20%28single-precision%29))
  (bind _maincharacterref (Variables|Default|GetMainCharacterRef))
  ;[1 1 1] Turn Up/Down
  (Class|PlayerController|AddPitchInput (select (and (Variables|/Game/Blueprints/FPS_MainCharacter_BP.FPS_MainCharacter_BP_C|GetisAiming _maincharacterref) (Utilities|Enum|Equal(Enum) (Variables|/Game/Blueprints/FPS_MainCharacter_BP.FPS_MainCharacter_BP_C|GetHasWeaponEquipedEnum _maincharacterref) "NewEnumerator1")) (/ AxisValue 3.0) AxisValue)))

(fn ConstructionScript)