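; Flashlight battery pickup actor that recharges the player's flashlight when collected.
; While the player character overlaps its sphere, the pickup binds its Pickup event to the character's Interact dispatcher and unbinds it on exit.
; On interact, it calls FlashlightCharging on the character reference cached at BeginPlay, then destroys itself.
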(event OnComponentBeginOverlap(Sphere)
  (params (OverlappedComponent :type Primitive%20Component%20Object%20Reference) (OtherActor :type Actor%20Object%20Reference) (OtherComp :type Primitive%20Component%20Object%20Reference) (OtherBodyIndex :type Integer) (bFromSweep :type Boolean) (SweepResult :type Hit%20Result%20Structure%20%28by%20ref%29))
  (bind _asfps_main_character_bp (Utilities|Casting|CastToFPS_MainCharacter_BP OtherActor))
  (EventDispatchers|AssignInteract _asfps_main_character_bp (delegate Custom|Pickup)))

(event OnComponentEndOverlap(Sphere)
  (params (OverlappedComponent :type Primitive%20Component%20Object%20Reference) (OtherActor :type Actor%20Object%20Reference) (OtherComp :type Primitive%20Component%20Object%20Reference) (OtherBodyIndex :type Integer))
  (bind _asfps_main_character_bp (Utilities|Casting|CastToFPS_MainCharacter_BP OtherActor))
  (EventDispatchers|UnbindEventfromInteract _asfps_main_character_bp (delegate Custom|Pickup)))

(event Custom|Pickup
  (Default|FlashlightCharging (Variables|Default|GetMainCharacterRef))
  (Actor|DestroyActor))

(event EventBeginPlay
  (bind _asfps_main_character_bp (Utilities|Casting|CastToFPS_MainCharacter_BP (Game|Player|GetPlayerPawn 0)))
  (Variables|Default|SetMainCharacterRef _asfps_main_character_bp))

(fn ConstructionScript)