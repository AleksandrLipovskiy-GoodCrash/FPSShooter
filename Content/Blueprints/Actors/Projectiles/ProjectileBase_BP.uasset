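; Base projectile actor that delivers damage and impact effects when its ProjectileMovement stops.
; It either sends a direct damage message to the hit actor or, for radius damage, messages overlapped actors using the ammo's radius and spawns an explosion impulse.
; The radius query ignores the player's current weapon.
; After either path, it hides the mesh, spawns the impact effect with the hit result and expires shortly afterward.
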(event OnProjectileStop(ProjectileMovement)
  (params (ImpactResult :type Hit%20Result%20Structure%20%28by%20ref%29))
  (CallFunction|ProjectileStop ImpactResult))

(event EventBeginPlay
  (bind _asfps_main_character_bp (Utilities|Casting|CastToFPS_MainCharacter_BP (Game|Player|GetPlayerPawn 0)))
  (Variables|Default|SetMainCharacterRef _asfps_main_character_bp))

(fn ConstructionScript)

(fn ProjectileStop
  (params (HitResult :type Hit%20Result%20Structure))
  (bind _projectilemesh (Variables|Default|GetProjectileMesh))
  (Utilities|FlowControl|Sequence
    (:then_0
      (if (Variables|Default|GetisCausingRadiusDamage)
        (CallFunction|ExplodeonImpact HitResult)
        (else
          (Class|TakeDamageBP|TakeDamage(Message) (.HitActor (Collision|BreakHitResult HitResult)) (Variables|Default|GetAmmoData) (Variables|Default|GetCriticalHitDamageModifier) HitResult))))
    (:then_1
      (Development|SetHiddeninGame _projectilemesh true false)
      (Game|SpawnActorfromClass (Variables|Default|GetImpactEffect) (Transformation|GetWorldTransform _projectilemesh) "AlwaysSpawn" 0 HitResult true 0)
      (Actor|SetLifeSpan 0.1))))

(fn ExplodeonImpact
  (params (HitResult :type Hit%20Result%20Structure))
  (bind _impactpoint (Collision|BreakHitResult HitResult))
  (Utilities|FlowControl|Sequence
    (:then_0
      (bind _outactors (Collision|SphereOverlapActors _impactpoint (.DamageRadius (Utilities|Struct|BreakAmmoData_BP (Variables|Default|GetAmmoData))) (Utilities|Array|MakeArray "ObjectTypeQuery2" "ObjectTypeQuery3") 0 (Utilities|Array|MakeArray (Variables|/Game/Blueprints/FPS_MainCharacter_BP.FPS_MainCharacter_BP_C|GetCurrentWeapon (Variables|Default|GetMainCharacterRef)))))
      (for _array_element _outactors
        (Class|TakeDamageBP|TakeDamageRadius(Message) _array_element HitResult (Variables|Default|GetAmmoData) (Variables|Default|GetCriticalHitDamageModifier))))
    (:then_1
      (Game|SpawnActorfromClass "/Game/Blueprints/Actors/Impulses/ExplosionImpulse_BP.ExplosionImpulse_BP_C" (Math|Transform|MakeTransform _impactpoint "0, 0, 0" "1,1,1") "AlwaysSpawn" 0 0))))