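; Base impact effect actor that plays surface-specific feedback at a hit point on BeginPlay.
; For blocking hits, the physical material's surface type selects particles and sound, with all flesh body-part surfaces sharing one set.
; Default and concrete surfaces also get a timed decal attached to the hit component, aligned to the normal with random roll.
; When IsUsingHitResult is false, it also spawns the default particles at the impact point.
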(event EventBeginPlay
  (bind _hitresult (Variables|Default|GetHitResult))
  (bind _hitresult_2 (Variables|Default|GetHitResult))
  (bind _decalsize (Variables|Default|GetDecalSize))
  (bind _fleshfx (Variables|Default|GetFleshFX))
  (bind _fleshsound (Variables|Default|GetFleshSound))
  (bind _normal (Collision|BreakHitResult _hitresult))
  (bind (_bblockinghit _binitialoverlap _time _distance _location _impactpoint _normal_2 _impactnormal _physmat _hitactor _hitcomponent _hitbonename) (Collision|BreakHitResult _hitresult_2))
  (bind _returnvalue (Math|Conversions|RotationFromXVector _normal))
  (bind _surfacetype (Variables|/Script/PhysicsCore.PhysicalMaterial|GetSurfaceType _physmat))
  (bind (_roll _pitch _yaw) (Math|Rotator|BreakRotator _returnvalue))
  (Utilities|FlowControl|Sequence
    (:then_0
      (Variables|Default|SetDecalRotation (Math|Rotator|MakeRotator (Math|Random|RandomFloatinRange -1.8e+02 1.8e+02) _pitch _yaw)))
    (:then_1
      (if _bblockinghit
        (Effects|SpawnEmitteratLocation (Utilities|Select :Index _surfacetype :SurfaceType_Default (Variables|Default|GetDefaultFX) :SurfaceType1 (Variables|Default|GetConcreteFX) :SurfaceType2 _fleshfx :SurfaceType3 _fleshfx :SurfaceType4 _fleshfx :SurfaceType5 _fleshfx :SurfaceType6 _fleshfx :SurfaceType7 _fleshfx :SurfaceType8 _fleshfx :SurfaceType9 _fleshfx :SurfaceType10 _fleshfx) _impactpoint)
        (Audio|PlaySoundatLocation (Utilities|Select :Index _surfacetype :SurfaceType_Default (Variables|Default|GetDefaultSound) :SurfaceType1 (Variables|Default|GetConcreteSound) :SurfaceType2 _fleshsound :SurfaceType3 _fleshsound :SurfaceType4 _fleshsound :SurfaceType5 _fleshsound :SurfaceType6 _fleshsound :SurfaceType7 _fleshsound :SurfaceType8 _fleshsound :SurfaceType9 _fleshsound :SurfaceType10 _fleshsound) _impactpoint "0, 0, 0" 1.0 1.0 0.0 0 0 0)
        (switch Utilities|FlowControl|Switch|SwitchonEPhysicalSurface _surfacetype
          (:SurfaceType_Default
            _)
          (:SurfaceType1
            _))
        (Class|GameplayStatics|SpawnDecalAttached (Utilities|Select :Index _surfacetype :SurfaceType_Default (Variables|Default|GetDefaultDecalMaterial) :SurfaceType1 (Variables|Default|GetConcreteDecalMaterial) :SurfaceType2 0) (Math|Vector|MakeVector _decalsize _decalsize _decalsize) _hitcomponent _hitbonename _impactpoint (Variables|Default|GetDecalRotation) "KeepWorldPosition" (Variables|Default|GetDecalLifeSpan))))
    (:then_2
      (if (not (Variables|Default|GetisUsingHitResult))
        (Effects|SpawnEmitteratLocation (Variables|Default|GetDefaultFX) _impactpoint)))))

(fn ConstructionScript)