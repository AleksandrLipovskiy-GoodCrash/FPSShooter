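; Base weapon pickup actor that lets the player acquire a weapon by interacting within its overlap sphere.
; Entering the sphere binds Pickup to the character's Interact dispatcher and shows the pickup HUD with the weapon's name and cost; leaving undoes both.
; Pickup asks the player character cached at BeginPlay to spawn the weapon, and destroys the actor only if that succeeds.
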(event OnComponentBeginOverlap(OverlapSphere)
  (params (OverlappedComponent :type Primitive%20Component%20Object%20Reference) (OtherActor :type Actor%20Object%20Reference) (OtherComp :type Primitive%20Component%20Object%20Reference) (OtherBodyIndex :type Integer) (bFromSweep :type Boolean) (SweepResult :type Hit%20Result%20Structure%20%28by%20ref%29))
  (bind _asfps_main_character_bp (Utilities|Casting|CastToFPS_MainCharacter_BP OtherActor))
  (EventDispatchers|AssignInteract _asfps_main_character_bp (delegate Custom|Pickup))
  (if (UserInterface|Viewport|IsinViewport (Variables|/Game/Blueprints/FPS_MainCharacter_BP.FPS_MainCharacter_BP_C|GetWeaponPickupHUDRef _asfps_main_character_bp))
    _
    (else
      (UserInterface|Viewport|AddtoViewport (Variables|/Game/Blueprints/FPS_MainCharacter_BP.FPS_MainCharacter_BP_C|GetWeaponPickupHUDRef _asfps_main_character_bp) 0)))
  (Default|UpdateData (Variables|/Game/Blueprints/FPS_MainCharacter_BP.FPS_MainCharacter_BP_C|GetWeaponPickupHUDRef _asfps_main_character_bp) (Variables|Default|GetWeaponName) (Variables|Default|GetWeaponCost)))

(event OnComponentEndOverlap(OverlapSphere)
  (params (OverlappedComponent :type Primitive%20Component%20Object%20Reference) (OtherActor :type Actor%20Object%20Reference) (OtherComp :type Primitive%20Component%20Object%20Reference) (OtherBodyIndex :type Integer))
  (bind _asfps_main_character_bp (Utilities|Casting|CastToFPS_MainCharacter_BP OtherActor))
  (EventDispatchers|UnbindEventfromInteract _asfps_main_character_bp (delegate Custom|Pickup))
  (Widget|RemovefromParent (Variables|/Game/Blueprints/FPS_MainCharacter_BP.FPS_MainCharacter_BP_C|GetWeaponPickupHUDRef _asfps_main_character_bp)))

(event Custom|Pickup
  (bind _isspawing (Default|SpawnWeapons (Variables|Default|GetMainCharacterRef) (Variables|Default|GetWeapon)))
  (if _isspawing
    (Actor|DestroyActor)))

(event EventBeginPlay
  (bind _asfps_main_character_bp (Utilities|Casting|CastToFPS_MainCharacter_BP (Game|Player|GetPlayerPawn 0)))
  (Variables|Default|SetMainCharacterRef _asfps_main_character_bp))

(fn ConstructionScript)